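; Steering-behavior agent that moves a physics-driven cone using seek, flee, pursuit, evade, wander, arrival or path following.
; Tick runs the behavior selected by AgentState, then turns the cone toward its velocity.
; Behaviors set a desired velocity, which feeds a force-scaled steering vector into the physics velocity, slowed within a radius for arrival.
; BP_Target actors found at BeginPlay serve as target and waypoints; pursuit and evade extrapolate TargetAgent's velocity.
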(event `self.ReceiveBeginPlay`
  ;[1 1 1] Begin Play
  (bind _output_get (set `self.CurrentVelocity` (10.0 10.0 10.0)))
  (`PrimitiveComponent.SetPhysicsLinearVelocity` (`self.Cone`) (* (`KismetMathLibrary.Normal` _output_get) (`self.MaxVelocity`)) true "None")
  (bind _returnvalue (`GameplayStatics.GetActorOfClass` "/Game/Blueprints/BP_Target.BP_Target_C"))
  (set `self.Target` _returnvalue)
  (bind _outactors (`GameplayStatics.GetAllActorsOfClass` "/Game/Blueprints/BP_Target.BP_Target_C"))
  (set `self.Targets` _outactors))

(event `self.ReceiveTick`
  (params (DeltaSeconds :type "Float (single-precision)"))
  (set `self.TargetPosition` (`SceneComponent.K2_GetComponentLocation` (`Actor.RootComponent` (`self.Target`))))
  (switch `/Game/Blueprints/Enum_AgentState` (`self.AgentState`)
    (:`NewEnumerator0`
      (`self.Seek` (`self.TargetPosition`)))
    (:`NewEnumerator1`
      (`self.Flee` (`self.TargetPosition`)))
    (:`NewEnumerator2`
      (`self.Pursuit` (`self.TargetAgent`)))
    (:`NewEnumerator5`
      (`self.Evade` (`self.TargetAgent`)))
    (:`NewEnumerator6`
      (`self.Wander`))
    (:`NewEnumerator7`
      (`self.PathFollowing`))
    (:`NewEnumerator8`
      (`self.Seek` (`self.TargetPosition`) true)))
  (`self.LookAtDirection`))

(fn `ApplyVelocity`
  (params (TargetPos :type "Vector Structure") (UseArrival :type Boolean))
  (locals (Distance :type "Float (double-precision)" :default 0.0))
  (bind _returnvalue (* (`KismetMathLibrary.Normal` (+ (`self.CurrentVelocity`) (`self.SteeringVelocity`))) (`self.MaxVelocity`)))
  (if UseArrival
    (set `local.Distance` (`KismetMathLibrary.Vector_Distance` (`SceneComponent.RelativeLocation` (`self.Cone`)) TargetPos))
    (if (< (`local.Distance`) (`self.SlowingRadius`))
      ;[1 1 1] Apply arrival
      (set `self.CurrentVelocity` (* _returnvalue (/ (`local.Distance`) (`self.SlowingRadius`))))
      (else
        (bind _output_get (set `self.CurrentVelocity` _returnvalue :!label _label))))
    (else
      (goto _label)))
  (`PrimitiveComponent.SetPhysicsLinearVelocity` (`self.Cone`) _output_get false "None"))

(fn `Evade`
  (params (TargetAgent :type "/Game/Blueprints/BP_Agent Object Reference"))
  (locals (FuturePosition :type "Vector Structure"))
  (bind _output_get (set `local.FuturePosition` (+ (`SceneComponent.RelativeLocation` (`/Game/Blueprints/BP_Agent.Cone` TargetAgent)) (`/Game/Blueprints/BP_Agent.CurrentVelocity` TargetAgent))))
  (`self.Flee` (+ _output_get (`SceneComponent.RelativeLocation` (`self.Cone`)))))

(fn `Flee`
  (params (Pos :type "Vector Structure"))
  (locals (TargetPos :type "Vector Structure"))
  (set `local.TargetPos` Pos)
  (`|ExecutionSequence`
    (:`then_0`
      ;[1 1 1] Set Desired Velocity
      (set `self.DesiredVelocity` (* (`KismetMathLibrary.Normal` (- (`SceneComponent.RelativeLocation` (`self.Cone`)) (`local.TargetPos`))) (`self.MaxVelocity`))))
    (:`then_1`
      (`self.SetSteeringVelocity`)
      (`self.ApplyVelocity` (`local.TargetPos`)))))

(fn `LookAtDirection`
  (`SceneComponent.K2_SetWorldRotation` (`self.Cone`) (`KismetMathLibrary.MakeRotator` (.roll (`KismetMathLibrary.FindLookAtRotation` (`SceneComponent.K2_GetComponentLocation` (`self.Cone`)) (+ (`self.CurrentVelocity`) (`SceneComponent.RelativeLocation` (`self.Cone`))))) (+ (.pitch (`KismetMathLibrary.FindLookAtRotation` (`SceneComponent.K2_GetComponentLocation` (`self.Cone`)) (+ (`self.CurrentVelocity`) (`SceneComponent.RelativeLocation` (`self.Cone`))))) -90.0) (.yaw (`KismetMathLibrary.FindLookAtRotation` (`SceneComponent.K2_GetComponentLocation` (`self.Cone`)) (+ (`self.CurrentVelocity`) (`SceneComponent.RelativeLocation` (`self.Cone`)))))) false false))

(fn `LookAtTarget`
  (params (TargetPos :type "Vector Structure")))

(fn `PathFollowing`
  (locals (target :type "Vector Structure"))
  (set `local.target` (`SceneComponent.K2_GetComponentLocation` (`Actor.RootComponent` (`|GetArrayItem` (`self.Targets`) (`self.currentTarget`)))))
  (if (< (`KismetMathLibrary.Vector_Distance` (`local.target`) (`SceneComponent.RelativeLocation` (`self.Cone`))) (`self.PathRadius`))
    (bind _result (`/Engine/EditorBlueprintResources/StandardMacros.IncrementInt` (`self.currentTarget`))
      (:`  `
        (set `self.currentTarget` _result)))
    (else
      (`self.Seek` (`local.target`)))))

(fn `Pursuit`
  (params (TargetAgent :type "/Game/Blueprints/BP_Agent Object Reference"))
  (locals (FuturePosition :type "Vector Structure"))
  (bind _output_get (set `local.FuturePosition` (+ (`SceneComponent.RelativeLocation` (`/Game/Blueprints/BP_Agent.Cone` TargetAgent)) (`/Game/Blueprints/BP_Agent.CurrentVelocity` TargetAgent))))
  (`self.Seek` (+ _output_get (`SceneComponent.RelativeLocation` (`self.Cone`)))))

(fn `Seek`
  (params (Pos :type "Vector Structure") (UseArrival :type Boolean))
  (locals (TargetPos :type "Vector Structure"))
  (set `local.TargetPos` Pos)
  (set `self.DesiredVelocity` (* (`KismetMathLibrary.Normal` (- (`local.TargetPos`) (`SceneComponent.RelativeLocation` (`self.Cone`)))) (`self.MaxVelocity`)))
  (`self.SetSteeringVelocity`)
  (`self.ApplyVelocity` (`local.TargetPos`) UseArrival))

(fn `SetSteeringVelocity`
  (set `self.SteeringVelocity` (* (`KismetMathLibrary.Normal` (- (`self.DesiredVelocity`) (`self.CurrentVelocity`))) (`self.MaxForce`))))

(fn `UserConstructionScript`)

(fn `Wander`
  (locals (CirclePosition :type "Vector Structure") (Angle :type "Float (double-precision)") (Displacement :type "Vector Structure" :default (0.0 -1.0 0.0)))
  (bind _anglestep (`self.AngleStep`))
  (`|ExecutionSequence`
    (:`then_0`
      ;[1 1 1] Set Circle Position
      (bind _output_get (set `local.CirclePosition` (`self.CurrentVelocity`)))
      (set `local.CirclePosition` (* (`KismetMathLibrary.Normal` _output_get) (`self.CircleDistance`))))
    (:`then_1`
      ;[1 1 1] Set Angle
      (set `local.Angle` (- (* (`KismetMathLibrary.RandomFloat`) _anglestep) (* _anglestep 0.5))))
    (:`then_2`
      ;[1 1 1] Set Displacement
      (set `local.Displacement` (`KismetMathLibrary.RotateAngleAxis` (* (`local.Displacement`) (`self.CircleDistance`)) (`local.Angle`))))
    (:`then_3`
      ;[1 1 1] Set Desired Velocity
      (set `self.DesiredVelocity` (+ (`local.CirclePosition`) (`local.Displacement`)))
      (`self.SetSteeringVelocity`)
      (`self.ApplyVelocity` (0.0 0.0 0.0)))))